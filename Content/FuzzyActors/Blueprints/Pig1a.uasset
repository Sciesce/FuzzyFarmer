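; Pig pawn Blueprint that wanders the navmesh around its spawn point.
; BeginPlay stores the starting location; Tick runs through a short Delay, then, if IsMoving is set, sends AIMoveTo to a random navigable point within a fixed radius of that start.
; A looping wander chain with randomized pauses is also present but disconnected, so it never runs.
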(event `self.ReceiveBeginPlay`
  (`|ExecutionSequence`
    (:`then_0`
      (set `self.startingLoc` (`self.K2_GetActorLocation`)))))

(event `self.ReceiveTick`
  (params (DeltaSeconds :type "Float (single-precision)"))
  (`KismetSystemLibrary.Delay` 2.0)
  (if (`self.isMoving`)
    (`|AIMoveTo` self (`NavigationSystemV1.K2_GetRandomLocationInNavigableRadius` (`self.startingLoc`) 5000.0 null null) null)))

(fn `UserConstructionScript`)