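; FuzzyPig is a collectible pig that wanders the navmesh around its spawn point.
; Tick, throttled by a random delay, sends it via AIMoveTo to random reachable points, with a flag blocking overlapping moves.
; Once the game has started, a ThirdPersonCharacter entering its box collects it.
; The pig then spawns a destructible DM_Pig in its place, blasts it with radial force and destroys itself.
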(event `self.ReceiveBeginPlay`
  (set `self.StartingLoc` (`self.K2_GetActorLocation`)))

(event `self.ReceiveTick`
  (params (DeltaSeconds :type "Float (single-precision)"))
  (`KismetSystemLibrary.Delay` (`KismetMathLibrary.RandomFloatInRange` 2.0 5.0))
  (if (not (`self.isMoving`))
    (set `self.isMoving` true)
    (`|AIMoveTo` self (`NavigationSystemV1.K2_GetRandomLocationInNavigableRadius` (`self.StartingLoc`) 5000.0 null null) null
      (:`OnSuccess`
        _)
      (:`OnFail`
        _))
    (set `self.isMoving` false)))

(event `self.Box.OnComponentBeginOverlap`
  (params (OverlappedComponent :type "PrimitiveComponent Object Reference") (OtherActor :type "Actor Object Reference") (OtherComp :type "PrimitiveComponent Object Reference") (OtherBodyIndex :type Integer) (bFromSweep :type Boolean) (SweepResult :type "HitResult Structure (by ref)"))
  (bind _asthird_person_character (cast `/Game/ThirdPersonBP/Blueprints/ThirdPersonCharacter` OtherActor))
  (if (`/Game/ThirdPersonBP/Blueprints/ThirdPersonCharacter.gameStarted` _asthird_person_character)
    (`PrimitiveComponent.SetCollisionEnabled` (`self.StaticMesh`) "NoCollision")
    (`/Game/ThirdPersonBP/Blueprints/ThirdPersonCharacter.collect_pig` _asthird_person_character)
    (bind _returnvalue (`|SpawnActorFromClass` "/Game/ThirdPersonBP/Blueprints/DM_Pig.DM_Pig_C" (`self.GetTransform`) "Undefined" "OverrideRootScale" null null))
    (`KismetSystemLibrary.Delay` 0.15)
    (`PrimitiveComponent.AddRadialForce` (`/Game/ThirdPersonBP/Blueprints/DM_Pig.Destructible` _returnvalue) (- (`self.K2_GetActorLocation`) (0.0 0.0 -50.0)) 300.0 50000.0 "RIF_Constant" false)
    (`self.K2_DestroyActor`)))

(fn `UserConstructionScript`)